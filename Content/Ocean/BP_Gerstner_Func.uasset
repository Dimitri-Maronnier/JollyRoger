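; Gerstner wave functions that compute ocean surface displacement at a given position.
; NewFunction0 evaluates one wave from direction, steepness, wavelength, speed, amplitude and real time, returning horizontal cosine and vertical sine offsets.
; NewFunction1 reads settings from the first OceanGlobalVariable actor found and sums four waves.
; Two use the base settings; two use negated directions with halved wavelength, speed and amplitude.
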(fn NewFunction0
  (params (Direction :type Vector) (Steepness :type Float%20%28single-precision%29) (NumWaves :type Float%20%28single-precision%29) (WaveLenght :type Float%20%28single-precision%29) (Speed :type Float%20%28single-precision%29) (Amplitude :type Float%20%28single-precision%29) (PositionOverSea :type Vector))
  (bind (_x _y) (Math|Vector|BreakVector PositionOverSea))
  (bind _returnvalue (Utilities|Time|GetRealTimeSeconds))
  (bind _returnvalue_2 (Math|Trig|GetPI))
  (bind (_x_2 _y_2) (Math|Vector|BreakVector Direction))
  (bind _returnvalue_3 (Math|Trig|GetPI))
  (bind _returnvalue_4 (Math|Vector2D|MakeVector2D _x _y))
  (bind _returnvalue_5 (Math|Vector2D|MakeVector2D _x_2 _y_2))
  (bind _returnvalue_6 (* _returnvalue_3 2.0))
  (bind _returnvalue_7 (* _returnvalue_2 2.0))
  (bind _returnvalue_8 (Math|Vector2D|Normalize2D _returnvalue_5))
  (bind _returnvalue_9 (/ _returnvalue_6 WaveLenght))
  (bind _returnvalue_10 (* _returnvalue_7 NumWaves))
  (bind _returnvalue_11 (Math|Vector2D|DotProduct(2D) _returnvalue_8 _returnvalue_4))
  (bind _returnvalue_12 (* Speed _returnvalue_9))
  (bind _returnvalue_13 (* _returnvalue_9 Amplitude))
  (bind _returnvalue_14 (* _returnvalue_11 _returnvalue_9))
  (bind _returnvalue_15 (* _returnvalue_13 _returnvalue_10))
  (bind _returnvalue_16 (* _returnvalue _returnvalue_12))
  (bind _returnvalue_17 (/ Steepness _returnvalue_15))
  (bind _returnvalue_18 (+ _returnvalue_14 _returnvalue_16))
  (bind _returnvalue_19 (Math|Trig|Cos(Radians) _returnvalue_18))
  (bind _returnvalue_20 (* _returnvalue_17 Amplitude))
  (return (Math|Vector|MakeVector (* (* _x_2 _returnvalue_19) _returnvalue_20) (* _returnvalue_20 (* _returnvalue_19 _y_2)) (* (Math|Trig|Sin(Radians) _returnvalue_18) (* Amplitude 2.0)))))

(fn NewFunction1
  (params (PositionOnSea :type Vector))
  (bind _outactors (Actor|GetAllActorsOfClass 0 "/Game/Ocean/OceanGlobalVariable.OceanGlobalVariable_C"))
  (for _array_element _outactors
    (bind _position (CallFunction|NewFunction0 (Utilities|Array|Get(acopy) (Variables|/Game/Ocean/OceanGlobalVariable.OceanGlobalVariable_C|GetDirection _array_element)) (Variables|/Game/Ocean/OceanGlobalVariable.OceanGlobalVariable_C|GetSteepness _array_element) (Variables|/Game/Ocean/OceanGlobalVariable.OceanGlobalVariable_C|GetNumWave _array_element) (Variables|/Game/Ocean/OceanGlobalVariable.OceanGlobalVariable_C|GetWaveLenght _array_element) (Variables|/Game/Ocean/OceanGlobalVariable.OceanGlobalVariable_C|GetSpeed _array_element) (Variables|/Game/Ocean/OceanGlobalVariable.OceanGlobalVariable_C|GetAmplitude _array_element) PositionOnSea))
    (bind _position_2 (CallFunction|NewFunction0 (Utilities|Array|Get(acopy) (Variables|/Game/Ocean/OceanGlobalVariable.OceanGlobalVariable_C|GetDirection _array_element) 1) (Variables|/Game/Ocean/OceanGlobalVariable.OceanGlobalVariable_C|GetSteepness _array_element) (Variables|/Game/Ocean/OceanGlobalVariable.OceanGlobalVariable_C|GetNumWave _array_element) (Variables|/Game/Ocean/OceanGlobalVariable.OceanGlobalVariable_C|GetWaveLenght _array_element) (Variables|/Game/Ocean/OceanGlobalVariable.OceanGlobalVariable_C|GetSpeed _array_element) (Variables|/Game/Ocean/OceanGlobalVariable.OceanGlobalVariable_C|GetAmplitude _array_element) PositionOnSea))
    (bind _position_3 (CallFunction|NewFunction0 (* (Utilities|Array|Get(acopy) (Variables|/Game/Ocean/OceanGlobalVariable.OceanGlobalVariable_C|GetDirection _array_element) 2) -1.0) (Variables|/Game/Ocean/OceanGlobalVariable.OceanGlobalVariable_C|GetSteepness _array_element) (Variables|/Game/Ocean/OceanGlobalVariable.OceanGlobalVariable_C|GetNumWave _array_element) (* (Variables|/Game/Ocean/OceanGlobalVariable.OceanGlobalVariable_C|GetWaveLenght _array_element) 0.5) (* (Variables|/Game/Ocean/OceanGlobalVariable.OceanGlobalVariable_C|GetSpeed _array_element) 0.5) (* (Variables|/Game/Ocean/OceanGlobalVariable.OceanGlobalVariable_C|GetAmplitude _array_element) 0.5) PositionOnSea))
    (bind _position_4 (CallFunction|NewFunction0 (* (Utilities|Array|Get(acopy) (Variables|/Game/Ocean/OceanGlobalVariable.OceanGlobalVariable_C|GetDirection _array_element) 3) -1.0) (Variables|/Game/Ocean/OceanGlobalVariable.OceanGlobalVariable_C|GetSteepness _array_element) (Variables|/Game/Ocean/OceanGlobalVariable.OceanGlobalVariable_C|GetNumWave _array_element) (* (Variables|/Game/Ocean/OceanGlobalVariable.OceanGlobalVariable_C|GetWaveLenght _array_element) 0.5) (* (Variables|/Game/Ocean/OceanGlobalVariable.OceanGlobalVariable_C|GetSpeed _array_element) 0.5) (* (Variables|/Game/Ocean/OceanGlobalVariable.OceanGlobalVariable_C|GetAmplitude _array_element) 0.5) PositionOnSea))
    (return (+ (+ _position _position_2) (+ _position_3 _position_4)))))